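; Skybox Blueprint whose construction script creates a dynamic StarField material on the skydome and sets its sun direction and color.
; An assigned directional light supplies both and derives SunHeight from pitch; otherwise SunHeight and actor yaw set direction, with color blended by height.
; Branches for sky colors, clouds, stars and curve-driven tinting are disconnected and never run.
; The Star Color Creator graph holds only unused RGB and magnitude-to-alpha conversion nodes.
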(fn `UserConstructionScript`
  (bind _sky_material (`self.Sky material`))
  (bind _sky_material_2 (`self.Sky material`))
  (bind _returnvalue (`PrimitiveComponent.CreateDynamicMaterialInstance` (`self.Skydome`) 0 "/Game/Materials/StarField.StarField"))
  (set `self.Sky material` _returnvalue)
  (if (`self.Refresh material`)
    _
    (else
      _))
  (set `self.Refresh material` false)
  (`/Engine/EditorBlueprintResources/StandardMacros.IsValid` (`self.Directional light actor`) ; Has a directional light been assigned?
    (:`Is Valid`
      (`MaterialInstanceDynamic.SetVectorParameterValue` _sky_material "Light direction" (`KismetMathLibrary.Conv_VectorToLinearColor` (`KismetMathLibrary.Conv_RotatorToVector` (`self.K2_GetActorRotation` (`self.Directional light actor`)))))
      (`MaterialInstanceDynamic.SetVectorParameterValue` _sky_material "Sun color" (`KismetMathLibrary.Conv_ColorToLinearColor` (`LightComponentBase.LightColor` (`Light.LightComponent` (`self.Directional light actor`)))))
      (set `self.Sun height` (`KismetMathLibrary.MapRange` (.pitch (`self.K2_GetActorRotation` (`self.Directional light actor`))) 0.0 -90.0 0.0 1.0)))
    (:`Is Not Valid`
      (`MaterialInstanceDynamic.SetVectorParameterValue` _sky_material_2 "Light direction" (`KismetMathLibrary.Conv_VectorToLinearColor` (`KismetMathLibrary.Conv_RotatorToVector` (`KismetMathLibrary.MakeRot` (`KismetMathLibrary.MapRange` (`self.Sun height`) -1.0 1.0 90.0 -90.0) (.yaw (`self.K2_GetActorRotation`))))))
      (`MaterialInstanceDynamic.SetVectorParameterValue` _sky_material_2 "Sun color" (`KismetMathLibrary.LinearColorLerp` (struct :`R` 1.0 :`G` 0.221 :`B` 0.04 :`A` 1.0) (struct :`R` 0.954 :`G` 0.901 :`B` 0.74412 :`A` 1.0) (`KismetMathLibrary.FClamp` (+ (`self.Sun height`) 0.2)))))))